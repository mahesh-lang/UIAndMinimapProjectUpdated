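; GameInfoInstance provides events that show the main menu and a message widget on screen with the mouse cursor visible.
; ShowMainMenu creates the menu from the NewWidget class if none is valid, caches it in MainMenuWB and adds it to the viewport.
; ShowMessageWidget follows the same pattern but never stores the widget it creates in the MessageWidget variable it checks.
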(event Custom|ShowMainMenu
  (bind _returnvalue (Game|GetPlayerController 0))
  (Utilities|IsValid (Variables|Default|GetMainMenuWB)
    (:Is%20Valid
      _)
    (:Is%20Not%20Valid
      (bind _returnvalue_2 (UserInterface|CreateWidget "/Game/ThirdPersonBP/NewWidget.NewWidget_C" _returnvalue))
      (Variables|Default|SetMainMenuWB _returnvalue_2)))
  (UserInterface|Viewport|AddtoViewport (Variables|Default|GetMainMenuWB) 0)
  (Variables|/Script/Engine.PlayerController|SetbShowMouseCursor _returnvalue true))

(event Custom|ShowMessageWidget
  (bind _returnvalue (Game|GetPlayerController 0))
  (Utilities|IsValid (Variables|Default|GetMessageWidget)
    (:Is%20Valid
      _)
    (:Is%20Not%20Valid
      (bind _returnvalue_2 (UserInterface|CreateWidget "/Game/ThirdPersonBP/MessageWidget.MessageWidget_C" _returnvalue))))
  (UserInterface|Viewport|AddtoViewport _returnvalue_2 0)
  (Variables|/Script/Engine.PlayerController|SetbShowMouseCursor _returnvalue true))