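; LobbyPC is a lobby player controller that relays chat messages between players.
; GetChatMessage pairs the incoming text with the sender's name from PlayerSettings, then loops over the LobbyGM game mode's AllPlayerControllers and calls UpdateChat on each LobbyPC.
; UpdateChat has no body yet, so received messages are not displayed by this graph.
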(event Custom|GetChatMessage
  (params (TextToSend :type Text))
  ;[1 1 1] Process incoming chat message and tells all player controllers to run update chat
  (Variables|Default|SetSenderText TextToSend)
  (Variables|Default|SetSenderName (.MyPlayerName (Utilities|Struct|BreakPlayerInfo (Variables|Default|GetPlayerSettings))))
  (bind _aslobby_gm (Utilities|Casting|CastToLobbyGM (Game|GetGameMode)))
  (for _array_element (Variables|/Game/Blueprints/Lobby/LobbyGM.LobbyGM_C|GetAllPlayerControllers _aslobby_gm)
    (bind _aslobby_pc (Utilities|Casting|CastToLobbyPC _array_element))
    (CallFunction|UpdateChat _aslobby_pc (Variables|Default|GetSenderName) (Variables|Default|GetSenderText))))

(event Custom|UpdateChat
  (params (Sender :type Text) (Text :type Text)))

(event EventBeginPlay)

(event EventTick
  (params (DeltaSeconds :type Float%20%28single-precision%29)))

(fn ConstructionScript)